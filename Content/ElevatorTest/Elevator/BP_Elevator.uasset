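; Elevator actor that moves toward one of five floor positions selected by the FloorLevel passed to MoveElevatortoTarget.
; Each call makes a single swept SetActorLocation step, using SetNewLocation to lerp from the current location to that floor's target vector.
; Tick only caches DeltaSeconds as the lerp alpha, so reaching a floor relies on repeated calls and slows on approach.
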(event `self.MoveElevatorToTarget`
  (params (FloorLevel :type "EET_FloorLevel Enum" :default "level_1"))
  (switch `EET_FloorLevel` FloorLevel
    (:`level_1`
      (bind _result (`self.SetNewLocation` (`self.Level 1`)))
      (`self.K2_SetActorLocation` _result true))
    (:`level_2`
      (bind _result_2 (`self.SetNewLocation` (`self.Level 2`)))
      (`self.K2_SetActorLocation` _result_2 true))
    (:`level_3`
      (bind _result_3 (`self.SetNewLocation` (`self.Level 3`)))
      (`self.K2_SetActorLocation` _result_3 true))
    (:`level_4`
      (bind _result_4 (`self.SetNewLocation` (`self.Level 4`)))
      (`self.K2_SetActorLocation` _result_4 true))
    (:`level_5`
      (bind _result_5 (`self.SetNewLocation` (`self.Level 5`)))
      (`self.K2_SetActorLocation` _result_5 true))))

(event `self.ReceiveTick`
  (params (DeltaSeconds :type "Float (single-precision)"))
  (set `self.Delta Seconds` DeltaSeconds))

(fn `SetNewLocation`
  (params (Target :type "Vector Structure"))
  (returns (Result :type "Vector Structure"))
  (return (`KismetMathLibrary.VLerp` (`self.K2_GetActorLocation`) Target (`self.Delta Seconds`))))

(fn `UserConstructionScript`)